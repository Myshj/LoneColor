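; Player controller that lets the player edit the material of the controlled pawn's plane through an on-screen controls widget.
; On BeginPlay it caches the pawn and its plane, creates a dynamic material instance and adds the widget with an update callback bound.
; Update functions copy widget values into base color, metallic, roughness and specular parameters.
; Escape flip-flops the widget between visible and collapsed.
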(event `self.ReceiveBeginPlay`
  (`self.InitMyPawn`)
  (`self.InitPlane`)
  (`self.InitMaterial`)
  (`self.InitControls`))

(event `Key|Escape`
  (params (Key :type "Key Structure"))
  (bind _controls (`self.Controls`))
  (:`Pressed`
    (`/Engine/EditorBlueprintResources/StandardMacros.FlipFlop`
      (:`A`
        (`Widget.SetVisibility` _controls "Visible"))
      (:`B`
        (`Widget.SetVisibility` _controls "Collapsed")))))

(fn `InitControls`
  (bind _returnvalue (`|CreateWidget` "/Game/Widgets/Controls.Controls_C" self))
  (bind _output_get (set `self.Controls` _returnvalue))
  (add `/Game/Widgets/Controls.Update` _output_get (`|CreateDelegate` :!event `UpdateMaterial`))
  (`UserWidget.AddToViewport` _output_get 0))

(fn `InitMaterial`
  (bind _returnvalue (`PrimitiveComponent.CreateDynamicMaterialInstance` (`StaticMeshActor.StaticMeshComponent` (`self.Plane`)) 0 "/Game/Materials/PlaneMaterial.PlaneMaterial" "None"))
  (set `self.PlaneMaterial` _returnvalue))

(fn `InitMyPawn`
  (bind _asmy_pawn (cast `/Game/Blueprints/MyPawn` (`self.K2_GetPawn`)))
  (set `self.MyPawn` _asmy_pawn))

(fn `InitPlane`
  (set `self.Plane` (`/Game/Blueprints/MyPawn.Plane` (`self.MyPawn`))))

(fn `UpdateColor`
  (bind _controls (`self.Controls`))
  (`MaterialInstanceDynamic.SetVectorParameterValue` (`self.PlaneMaterial`) "Base Color" (make `LinearColor` (`SpinBox.GetValue` (`/Game/Widgets/Controls.ColorRed` _controls)) (`SpinBox.GetValue` (`/Game/Widgets/Controls.ColorGreen` _controls)) (`SpinBox.GetValue` (`/Game/Widgets/Controls.ColorBlue` _controls)) (`SpinBox.GetValue` (`/Game/Widgets/Controls.ColorAlpha` _controls)))))

(fn `UpdateMaterial`
  (`self.UpdateColor`)
  (`self.UpdateMetallic`)
  (`self.UpdateRoughness`)
  (`self.UpdateSpecular`))

(fn `UpdateMetallic`
  (`MaterialInstanceDynamic.SetScalarParameterValue` (`self.PlaneMaterial`) "Metallic" (`SpinBox.GetValue` (`/Game/Widgets/Controls.Metallic` (`self.Controls`)))))

(fn `UpdateRoughness`
  (`MaterialInstanceDynamic.SetScalarParameterValue` (`self.PlaneMaterial`) "Roughness" (`SpinBox.GetValue` (`/Game/Widgets/Controls.Roughness` (`self.Controls`)))))

(fn `UpdateSpecular`
  (`MaterialInstanceDynamic.SetScalarParameterValue` (`self.PlaneMaterial`) "Specular" (`SpinBox.GetValue` (`/Game/Widgets/Controls.Specular` (`self.Controls`)))))

(fn `UserConstructionScript`)